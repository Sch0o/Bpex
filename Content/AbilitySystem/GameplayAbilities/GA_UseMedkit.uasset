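; Gameplay ability that uses a medkit from an inventory slot to heal its owner.
; It is triggered by a gameplay event carrying the target character, the slot index as magnitude, and the item data as optional object.
; After waiting the item's use duration, it consumes one item from that slot, applies the medkit heal effect and ends the ability.
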(event Ability|EventActivateAbility)

(event Ability|EventActivateAbilityFromEvent
  (params (EventData :type Gameplay%20Event%20Data%20Structure%20%28by%20ref%29))
  (bind (_eventtag _instigator _target _optionalobject _optionalobject2 _contexthandle _instigatortags _targettags _eventmagnitude) (Utilities|Struct|BreakGameplayEventData EventData))
  (Development|PrintString "Using Medkit")
  (Variables|Default|SetMyCharacter _target)
  (Variables|Default|SetCurrentSlotIndex (Math|Float|Round _eventmagnitude))
  (bind _asinventory_item_data (Utilities|Casting|CastToInventoryItemData _optionalobject))
  (Ability|Tasks|WaitDelay (Variables|/Script/Bpex.InventoryItemData|GetUseDuration _asinventory_item_data)
    (:OnFinish
      (Class|InventoryComponent|ConsumeIteminSlot (Actor|GetComponentbyClass (Variables|Default|GetMyCharacter) "/Script/Bpex.InventoryComponent") (Variables|Default|GetCurrentSlotIndex) 1)
      (Ability|ApplyGameplayEffectToOwner "/Game/AbilitySystem/GameEffects/GE_Heal_Medkit.GE_Heal_Medkit_C")
      (Ability|EndAbility)
      (Development|PrintString "Fnish Using Medkit"))))